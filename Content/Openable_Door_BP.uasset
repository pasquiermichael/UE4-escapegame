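; Openable door actor that swings 90 degrees in yaw from its starting rotation when its OpenDoor member receives an open request.
; BeginPlay caches the initial rotation, and a timeline curve drives the yaw interpolation, setting pitch and roll to zero.
; An event track on the timeline plays the door lock sound at the actor's location.
; Close requests reverse the same timeline.
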(event `self.ReceiveBeginPlay`
  (set `self.InitialRotation` (`self.K2_GetActorRotation`)))

(event `self.OpenDoor.OnOpenRequest`
  (bind _initialrotation (`self.InitialRotation`))
  (bind (_direction _openanglecurve) (`Timeline|Timeline_0` :!label _label)
    (:`Update`
      (`self.K2_SetActorRotation` (`KismetMathLibrary.MakeRotator` 0.0 0.0 (`KismetMathLibrary.Lerp` (.yaw _initialrotation) (.yaw (`KismetMathLibrary.ComposeRotators` _initialrotation (`KismetMathLibrary.MakeRotator` 0.0 0.0 90.0))) _openanglecurve))))
    (:`EventAngleTrack`
      (`GameplayStatics.PlaySoundAtLocation` "/Game/Audio/door-lock.door-lock" (`self.K2_GetActorLocation`) (struct) 1.0 1.0 0.0 null null null))))

(event `self.OpenDoor.OnCloseRequest`
  (goto _label :!via `Reverse`))

(fn `UserConstructionScript`)